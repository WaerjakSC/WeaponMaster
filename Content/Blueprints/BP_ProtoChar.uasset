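; Prototype player character with a dash, pause menu and fox companion.
; BeginPlay creates the UI widgets, starts camera occluder fading and caches the fox.
; Tick feeds air time to the anim instance, clears the dash flag outside flying mode and makes the fox follow in StartArea; a retriggerable delay ends dashes.
; Death plays a fade, moves the player to the GameMode's respawn location, respawns the fox and resets widgets.
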(event Custom|PlayerDied
  ;[1 1 1] Respawn Logic
  (UserInterface|Animation|PlayAnimation (Variables|Default|GetDied) (Variables|Default|GetFadeBlack (Variables|Default|GetDied)) 0.0 1 "Forward" 1.0)
  (Utilities|FlowControl|Delay 0.75)
  (bind _asbp_comet_game_mode (Utilities|Casting|CastTo (Game|GetGameMode)))
  (Transformation|SetActorLocation (Variables|Default|GetRespawnLocation _asbp_comet_game_mode) false false)
  (bind _asnew_main_anim_bp (Utilities|Casting|CastTo (Components|SkeletalMesh|GetAnimInstance (Variables|Character|GetMesh))))
  (Variables|Default|SetDied _asnew_main_anim_bp true)
  (bind _asbp_owl_controller (Utilities|Casting|CastTo (Game|GetPlayerController 0)))
  (CallFunction|ResetWidget _asbp_owl_controller)
  (bind _asbp_fox_ai (Utilities|Casting|CastTo (Variables|Default|GetFoxFriend)))
  (CallFunction|Respawn _asbp_fox_ai)
  (Utilities|FlowControl|Delay 5.0)
  (bind _outactors (Actor|GetAllActorsOfClass 0))
  (for _array_element _outactors
    (bind _asbp_wolf_ai (Utilities|Casting|CastTo _array_element))
    (CallFunction|ResetWidgetAI _asbp_wolf_ai)))

(event Custom|Tick2
  ;[1 1 1] Fox Tick
  (if (Utilities|Enum|Equal(Enum) (Variables|Default|GetLevelName) "StartArea")
    (bind _asbp_fox_ai (Utilities|Casting|CastTo (Variables|Default|GetFoxFriend)))
    (CallFunction|FollowChar _asbp_fox_ai)))

(event EventBeginPlay
  ;[1 1 1] Set up all the widgets
  (bind _returnvalue (UserInterface|CreateWidget 0))
  (Variables|Default|SetWidget%20Ref _returnvalue)
  (bind _returnvalue_2 (UserInterface|CreateWidget 0))
  (bind _output_get (Variables|Default|SetCharUI _returnvalue_2))
  (UserInterface|Viewport|AddtoViewport _output_get 0)
  (bind _returnvalue_3 (UserInterface|CreateWidget 0))
  (bind _output_get_2 (Variables|Default|SetDied _returnvalue_3))
  (UserInterface|Viewport|AddtoViewport _output_get_2 0)
  (CallFunction|Init (Variables|Default|GetFadeCameraOccluders) (Variables|Default|GetCamera) (Variables|Default|GetCapsuleComponent))
  (bind _outactors (Actor|GetAllActorsOfClass 0))
  (Variables|Default|SetFoxFriend (Utilities|Array|Get(acopy) _outactors)))

(event EventStartTimer
  ;[1 1 1] Dash animation logic
  (bind _asnew_main_anim_bp (Utilities|Casting|CastTo (Components|SkeletalMesh|GetAnimInstance (Variables|Character|GetMesh))))
  (Variables|Default|SetIsDashing? _asnew_main_anim_bp true)
  (Audio|PlaySound2D 0)
  (Utilities|FlowControl|RetriggerableDelay (Variables|Default|GetDashDuration))
  (if (Class|NavMovementComponent|IsFlying (Variables|Character|GetCharacterMovement))
    (CallFunction|StopDash)
    (bind _asnew_main_anim_bp_2 (Utilities|Casting|CastTo (Components|SkeletalMesh|GetAnimInstance (Variables|Character|GetMesh))))
    (Variables|Default|SetIsDashing? _asnew_main_anim_bp_2 false)
    (CallFunction|Tick2)))

(event EventTick
  (params (DeltaSeconds :type Float%20%28single-precision%29))
  (bind _charactermovement (Variables|Character|GetCharacterMovement))
  ;[1 1 1] Dash animation logic
  (if (AI|Components|NavMovement|IsFalling _charactermovement)
    (bind _asnew_main_anim_bp (Utilities|Casting|CastTo (Components|SkeletalMesh|GetAnimInstance (Variables|Character|GetMesh))))
    (Variables|Default|SetTime%20in%20Air _asnew_main_anim_bp (+ DeltaSeconds (Variables|Default|GetTime%20in%20Air _asnew_main_anim_bp))))
  (if (not (Class|NavMovementComponent|IsFlying _charactermovement))
    (bind _asnew_main_anim_bp_2 (Utilities|Casting|CastTo (Components|SkeletalMesh|GetAnimInstance (Variables|Character|GetMesh))))
    (Variables|Default|SetIsDashing? _asnew_main_anim_bp_2 false)
    (CallFunction|Tick2)))

(event Input|ActionEvents|InputActionPause
  (params (Key :type Key%20Structure))
  (bind _widget_ref (Variables|Default|GetWidget%20Ref))
  (bind _startmenuwidget (Variables|Default|GetStartMenuWidget))
  (:Pressed
    (Utilities|IsValid _startmenuwidget
      (:Is%20Valid
        (if (not (UserInterface|Viewport|IsinViewport _startmenuwidget))
          (CallFunction|PauseGame :!label _label)
          (if (UserInterface|Viewport|IsinViewport _widget_ref)
            (Widget|RemovefromParent _widget_ref)
            (else
              (UserInterface|Viewport|AddtoViewport _widget_ref 0)))))
      (:Is%20Not%20Valid
        (goto _label)))))

(fn ConstructionScript)