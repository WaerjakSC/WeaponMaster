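; Weight trigger template actor that works as a pressure plate, moving vertically on overlap and activating another Blueprint object.
; Begin overlap at the start height calls OpenSesame on the target and plays a Down timeline offsetting Z from StartPos.
; End overlap at the lowered height calls CloseSesame and plays an Up timeline.
; Targets come from index 1 of GetAllActorsOfClass, and exact Z comparisons gate both moves.
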(event EventBeginPlay)

(event Collision|EventActorBeginOverlap
  (params (OtherActor :type Actor%20Object%20Reference))
  (bind _startpos (Variables|Default|GetStartPos))
  ;[1 1 1] Move actor up or down smoothly
  (if (== (.z (Transformation|GetActorLocation)) (.z (Variables|Default|GetStartPos)))
    ;;[1 1 1] Calls a blueprint event to activate another blueprint object
    (bind _outactors (Actor|GetAllActorsOfClass 0))
    (CallFunction|OpenSesame (Utilities|Array|Get(acopy) _outactors 1))
    (bind _down (Timeline|Timeline_0 PlayFromStart)
      (:Update
        (Transformation|SetActorLocation (Math|Vector|MakeVector (.x _startpos) (.y _startpos) (+ _down (.z _startpos))) false false)))))

(event Collision|EventActorEndOverlap
  (params (OtherActor :type Actor%20Object%20Reference))
  (bind _startpos (Variables|Default|GetStartPos))
  ;[1 1 1] Move actor up or down smoothly
  (if (== (.z (Transformation|GetActorLocation)) (- (.z (Variables|Default|GetStartPos)) 25.0))
    ;;[1 1 1] Calls a blueprint event to activate another blueprint object
    (bind _outactors (Actor|GetAllActorsOfClass 0))
    (CallFunction|CloseSesame (Utilities|Array|Get(acopy) _outactors 1))
    (bind _up (Timeline|Timeline_1 PlayFromStart)
      (:Update
        (Transformation|SetActorLocation (Math|Vector|MakeVector (.x _startpos) (.y _startpos) (+ _up (.z _startpos))) false false)))))

(fn ConstructionScript)