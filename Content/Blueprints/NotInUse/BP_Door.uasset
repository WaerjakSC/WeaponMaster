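; Door Blueprint, filed under NotInUse, that rotates its static mesh about the roll axis when a switch calls it.
; OpenSesame and CloseSesame each check the actor's roll against their end angle, then play a timeline that drives the mesh's relative roll.
; The timeline names are reversed relative to the events: OpenSesame plays Close and CloseSesame plays Open.
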(event Custom|Open%20Sesame
  ;[1 1 1] Events called from Switch to rotate actor
  (if (!= (.roll (Transformation|GetActorRotation)) 9e+01)
    (bind _newtrack_0 (Timeline|Close PlayFromStart)
      (:Update
        (Transformation|SetRelativeRotation (Variables|Debug|GetStaticMeshComponent) (Math|Rotator|MakeRotator _newtrack_0 0.0 0.0) false false)))))

(event Custom|Close%20Sesame
  ;[1 1 1] Events called from Switch to rotate actor
  (if (!= (.roll (Transformation|GetActorRotation)) 0.0)
    (bind _newtrack_0 (Timeline|Open PlayFromStart)
      (:Update
        (Transformation|SetRelativeRotation (Variables|Debug|GetStaticMeshComponent) (Math|Rotator|MakeRotator _newtrack_0 0.0 0.0) false false)))))

(event EventBeginPlay)

(fn ConstructionScript)