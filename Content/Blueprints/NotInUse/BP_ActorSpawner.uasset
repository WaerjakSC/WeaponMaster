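; BP_ActorSpawner is an actor spawner, filed under NotInUse, that times spawn calls whose logic lives outside this graph.
; OpenSesame and CloseSesame toggle a spawn flag that gates the Trapped event.
; Trapped waits, then runs either the constant spawner or two staggered spawns, resetting the delay for later calls.
; BPStaggered runs the same staggered sequence without checking the flag.
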(event Custom|Open%20Sesame
  (Variables|Default|SetSpawnNow true))

(event Custom|Close%20Sesame
  (Variables|Default|SetSpawnNow false))

(event EventBeginPlay)

(event Collision|EventActorBeginOverlap
  (params (OtherActor :type Actor%20Object%20Reference)))

(event EventTick
  (params (DeltaSeconds :type Float%20%28single-precision%29)))

(event EventTrapped
  (if (Variables|Default|GetSpawnNow)
    (if (Variables|Default|GetStaggeredSpawns)
      (Utilities|FlowControl|Delay (Variables|Default|GetDelay))
      (CallFunction|StaggeredSpawningOne)
      (Variables|Default|SetDelay 4.0)
      (Utilities|FlowControl|Delay 2.0)
      (CallFunction|StaggeredSpawningTwo)
      (else
        (Utilities|FlowControl|Delay (Variables|Default|GetDelay))
        (CallFunction|ConstantSpawner)
        (Variables|Default|SetDelay 4.0)))))

(event EventBPStaggered
  (Utilities|FlowControl|Delay (Variables|Default|GetDelay))
  (CallFunction|StaggeredSpawningOne)
  (Variables|Default|SetDelay 4.0)
  (Utilities|FlowControl|Delay 2.0)
  (CallFunction|StaggeredSpawningTwo))

(fn ConstructionScript)