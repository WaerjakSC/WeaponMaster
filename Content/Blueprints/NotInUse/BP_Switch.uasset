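; BP_Switch is a usable lever that opens or closes a target actor once the player has the required potatoes.
; OnUsed calls Used, which requires an exact potato count on the player controller, otherwise printing a warning.
; A makeshift one-second delay curbs spamming after first use.
; Timelines pitch the switch, and each update sets OnOff and calls OpenSesame or CloseSesame on the first actor found by class.
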(event Custom|Used
  (bind _returnvalue (Transformation|GetActorRotation))
  ;[1 1 1] Checks if Player has enough potatoes
  (bind _asowl_controller (Utilities|Casting|CastTo (Game|GetPlayerController 0)))
  (if (== (Variables|Default|GetPotatoes _asowl_controller) (Variables|Keys|GetRequired%20Potatoes))
    ;[1 1 1] Hackneyed way to stop player from spamming Use (refactor later)
    (if (Variables|SwitchStatus|GetNoDelay)
      (Utilities|FlowControl|Delay 1.0)
      (else
        (Variables|SwitchStatus|SetNoDelay true)))
    (if (Variables|Default|GetOnOff)
      ;[1 1 1] Rotate 45 degrees up or down depending on on/off status
      (bind _switch_rotation (Timeline|Rotation%20Timeline PlayFromStart)
        (:Update
          (Transformation|SetActorRelativeRotation (Math|Rotator|MakeRotator (.roll _returnvalue) (.pitch (Math|Rotator|MakeRotator 0.0 _switch_rotation 0.0)) (.yaw _returnvalue)))
          (Variables|Default|SetOnOff false)
          (bind _outactors (Actor|GetAllActorsOfClass 0))
          (CallFunction|CloseSesame (Utilities|Array|Get(acopy) _outactors))))
      (else
        (bind _rotate (Timeline|RotationOff PlayFromStart)
          (:Update
            (Transformation|SetActorRelativeRotation (Math|Rotator|MakeRotator (.roll _returnvalue) (.pitch (Math|Rotator|MakeRotator 0.0 _rotate 0.0)) (.yaw _returnvalue)))
            (Variables|Default|SetOnOff true)
            (bind _outactors_2 (Actor|GetAllActorsOfClass 0))
            (CallFunction|OpenSesame (Utilities|Array|Get(acopy) _outactors_2))))))
    (else
      (Development|PrintText "Not enough Potatoes!" true false "(R=1.000000,G=0.032358,B=0.000000,A=1.000000)"))))

(event EventBeginPlay)

(event Collision|EventActorBeginOverlap
  (params (OtherActor :type Actor%20Object%20Reference)))

(event EventTick
  (params (DeltaSeconds :type Float%20%28single-precision%29)))

(fn ConstructionScript)

(fn OnUsed
  (params (character :type Character%20Object%20Reference))
  (CallFunction|Used)
  (return false))