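; NextLevel is a level exit actor that activates once the game mode's WinCondition is true and advances the player through the levels.
; Tick polls that flag to switch on rune particles and hide a linked decal.
; An overlap then triggers a light beam, character UI fade to black and sound.
; After a delay, Desert opens Forest, Forest shows a widget and pauses, and any other level opens Desert.
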(event EventBeginPlay)

(event Collision|EventActorBeginOverlap
  (params (OtherActor :type Actor%20Object%20Reference))
  (bind _asbp_comet_game_mode (Utilities|Casting|CastTo (Game|GetGameMode)))
  (if (Variables|Default|GetWinCondition _asbp_comet_game_mode)
    (Components|Activation|SetActive (Variables|Default|GetLightBeam) true false)
    (bind _asbp_proto_char (Utilities|Casting|CastTo (Game|GetPlayerCharacter 0)))
    (UserInterface|Animation|PlayAnimation (Variables|Default|GetCharUI _asbp_proto_char) (Variables|Default|GetFadeToBlack (Variables|Default|GetCharUI _asbp_proto_char)) 0.0 1 "Forward" 1.0)
    (Audio|PlaySound2D 0)
    (Utilities|FlowControl|Delay 2.0)
    (bind _returnvalue (Game|GetCurrentLevelName true))
    (if (Utilities|Enum|Equal(Enum) _returnvalue "Forest")
      (bind _returnvalue_2 (UserInterface|CreateWidget 0))
      (UserInterface|Viewport|AddtoViewport _returnvalue_2 0)
      (Game|SetGamePaused true)
      (else
        ;[1 1 1] Open new level
        (bind _returnvalue_3 (Game|GetCurrentLevelName true))
        (if (Utilities|Enum|Equal(Enum) _returnvalue_3 "Desert")
          (Game|OpenLevel(byName) "Forest")
          (else
            (Game|OpenLevel(byName) "Desert")))))))

(event EventTick
  (params (DeltaSeconds :type Float%20%28single-precision%29))
  (bind _decalactor (Variables|Default|GetDecalActor))
  (bind _asbp_comet_game_mode (Utilities|Casting|CastTo (Game|GetGameMode)))
  (if (Variables|Default|GetWinCondition _asbp_comet_game_mode)
    (Components|Activation|SetActive (Variables|Default|GetRuneParticles) true false)
    (if (Utilities|IsValid _decalactor)
      (Rendering|SetVisibility (Variables|/Script/Engine.DecalActor|GetDecal _decalactor) false false)
      (else
        (Development|PrintText "DecalActor is not set to a valid object" true false "(R=1.000000,G=0.032358,B=0.000000,A=1.000000)")))))

(fn ConstructionScript)