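; Pickup actor that rotates through a timeline to signal it can be collected and can activate a separate Crystal actor.
; StartMovement plays a sound, calls CrystalActivated on the Crystal, then raises it from its start point with a timeline.
; Two further timelines chain through their Finished pins to bob the Crystal up and down, re-capturing its location as the base for offsets.
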(event EventStartMovement
  (bind _crystal (Variables|Default|GetCrystal))
  (bind _returnvalue (Transformation|GetActorLocation _crystal))
  (Audio|PlaySound2D 0)
  (bind _asbp_small_crystal (Utilities|Casting|CastTo (Variables|Default|GetCrystal)))
  (CallFunction|CrystalActivated _asbp_small_crystal)
  ;[1 1 1] Moves the crystal up from its original position
  (bind _new_location (Timeline|Move%20Platform Play)
    (:Update
      (Transformation|SetActorLocation (Variables|Default|GetCrystal) (Math|Vector|MakeVector (.x (Variables|Default|GetStartPoint)) (.y (Variables|Default|GetStartPoint)) (+ (.z (Variables|Default|GetStartPoint)) _new_location)) false false))
    (:Finished
      ;[1 1 1] Logic for alternating movement up or down
      (Variables|Default|SetStartPoint _returnvalue)
      (bind _bobup (Timeline|MoveUp Play)
        (:Update
          (Transformation|SetActorLocation _crystal (Math|Vector|MakeVector (.x (Variables|Default|GetStartPoint)) (.y (Variables|Default|GetStartPoint)) (+ _bobup (.z (Variables|Default|GetStartPoint)))) false false))
        (:Finished
          (Variables|Default|SetEndPoint _returnvalue)
          (bind _bobdown (Timeline|MoveDown PlayFromStart)
            (:Update
              (Transformation|SetActorLocation _crystal (Math|Vector|MakeVector (.x (Variables|Default|GetEndPoint)) (.y (Variables|Default|GetEndPoint)) (+ _bobdown (.z (Variables|Default|GetEndPoint)))) false false))
            (:Finished
              (Timeline|MoveUp PlayFromStart))))))))

(event EventRotateActor
  ;[1 1 1] Rotate the item to signify it can be picked up
  (bind _rotate (Timeline|RotateItem PlayFromStart)
    (:Update
      (Transformation|SetActorRotation (Math|Rotator|MakeRotator 0.0 0.0 _rotate)))))

(fn ConstructionScript)